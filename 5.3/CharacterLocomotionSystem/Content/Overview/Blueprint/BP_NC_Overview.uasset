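; Reference overview Blueprint for a character using NewCharacterMovementComponent, laying out its extended movement API rather than adding gameplay.
; Custom advanced and extended movement overrides only call the parent, while the movement data getters return empty.
; Each move, from sprint, vault and slide to wall run, climb, fly and swim, has its own graph of empty event hooks and unconnected action, check and tuning nodes.
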(fn ConstructionScript)

(fn CanCustomAdvancedMovement
  (return (|CallParentFunction)))

(fn GetCustomAdvancedMovementData
  (return 0))

(fn GetClimbUpData
  (return 0))

(fn GetMantleData
  (return 0))

(fn GetVaultData
  (return 0))

(fn StartCustomAdvancedMovement
  (bind _returnvalue (|CallParentFunction))
  (return _returnvalue))

(fn GetMaxCustomAdvancedSpeed
  (return (|CallParentFunction)))

(fn GetMaxCustomExtendedSpeed
  (return (|CallParentFunction)))

(fn CanCustomExtendedMovement
  (return (|CallParentFunction)))

(fn StartCustomExtendedMovement
  (bind _returnvalue (|CallParentFunction))
  (return _returnvalue))

(fn GetMaxCustomExtendedAcceleration
  (return (|CallParentFunction)))

(fn GetMaxCustomExtendedDeceleration
  (return (|CallParentFunction)))

(event EventEnterCustomExtendedMovement
  (|CallParentFunction))

(event EventExitCustomExtendedMovement
  (|CallParentFunction))

(event EventCustomExtendedMovementPhysics
  (params (deltaTime :type Float%20%28single-precision%29) (Iterations :type Integer))
  (|CallParentFunction deltaTime Iterations))

(event EventStopCustomExtendedMovement
  (|CallParentFunction))

(event OnSprintStart(NewCharacterMovementComponent))

(event OnSprintStop(NewCharacterMovementComponent))

(event OnCustomAdvancedMovementStart(NewCharacterMovementComponent)
  (params (CurrentWall :type Current%20Wall%20Info%20Structure)))

(event OnCustomAdvancedMovementInitialized(NewCharacterMovementComponent)
  (params (CustommovementData :type Advanced%20Movement%20Primary%20Data%20Asset%20Object%20Reference)))

(event OnCustomAdvancedMovementStop(NewCharacterMovementComponent))

(event EventAddandUpdateCustomAdvancedWarpTargets
  (|CallParentFunction))

(event EventStopCustomAdvancedMovement
  (|CallParentFunction))

(event EventEnterCustomAdvancedMovement
  (|CallParentFunction))

(event EventCustomAdvancedMovementPhysics
  (params (deltaTime :type Float%20%28single-precision%29) (Iterations :type Integer))
  (|CallParentFunction deltaTime Iterations))

(event EventExitCustomAdvancedMovement
  (|CallParentFunction))

(event OnVaultStart(NewCharacterMovementComponent)
  (params (CurrentWall :type Current%20Wall%20Info%20Structure)))

(event OnVaultStop(NewCharacterMovementComponent))

(event OnVaultInitialize(NewCharacterMovementComponent)
  (params (VaultData :type Vault%20Primary%20Data%20Asset%20Object%20Reference)))

(event OnMantleStart(NewCharacterMovementComponent)
  (params (CurrentWall :type Current%20Wall%20Info%20Structure)))

(event OnMantleStop(NewCharacterMovementComponent))

(event OnMantleInitialize(NewCharacterMovementComponent)
  (params (MantleData :type Mantle%20Primary%20Data%20Asset%20Object%20Reference)))

(event OnClimbUpStart(NewCharacterMovementComponent)
  (params (CurrentWall :type Current%20Wall%20Info%20Structure)))

(event OnClimbUpStop(NewCharacterMovementComponent))

(event OnClimbUpInitialize(NewCharacterMovementComponent)
  (params (ClimbUpData :type Climb%20Up%20Primary%20Data%20Asset%20Object%20Reference)))

(event OnCrouchSprintStart(NewCharacterMovementComponent))

(event OnCrouchSprintStop(NewCharacterMovementComponent))

(event OnProneStart(NewCharacterMovementComponent))

(event OnProneStop(NewCharacterMovementComponent))

(event OnSlideStart(NewCharacterMovementComponent))

(event OnSlideStop(NewCharacterMovementComponent))

(event OnDashStart(NewCharacterMovementComponent)
  (params (TargetLocation :type Vector :default "0, 0, 0")))

(event OnDashStop(NewCharacterMovementComponent))

(event OnWallRunStart(NewCharacterMovementComponent)
  (params (CurrentWall :type Current%20Wall%20Info%20Structure)))

(event OnWallRunStop(NewCharacterMovementComponent))

(event OnClimbStart(NewCharacterMovementComponent)
  (params (CurrentWall :type Current%20Wall%20Info%20Structure)))

(event OnClimbStop(NewCharacterMovementComponent))

(event OnClimbReachedUpLedge(NewCharacterMovementComponent)
  (params (CurrentWall :type Current%20Wall%20Info%20Structure)))

(event OnFlyStart(NewCharacterMovementComponent))

(event OnFlyStop(NewCharacterMovementComponent))

(event OnFastFlyStart(NewCharacterMovementComponent))

(event OnFastFlyStop(NewCharacterMovementComponent))

(event OnFastSwimStart(NewCharacterMovementComponent))

(event OnFastSwimStop(NewCharacterMovementComponent))